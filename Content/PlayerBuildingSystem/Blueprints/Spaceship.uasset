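; Pilotable spaceship pawn that the building character can board and leave.
; Overlapping it binds the character's ShipInteract event so the player controller possesses the ship and hides the character, and leaving the overlap unbinds it.
; While piloting, axis inputs drive forward movement and yaw turning, W plays the Thruster, and E moves the character to the JumpOut point, repossesses and unhides it.
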(event `self.ReceiveActorBeginOverlap`
  (params (OtherActor :type "Actor Object Reference"))
  (bind _asbuilding_character (cast `/Game/PlayerBuildingSystem/Blueprints/BuildingCharacter` OtherActor))
  (bind _output_get (set `self.Player` _asbuilding_character))
  (add `/Game/PlayerBuildingSystem/Blueprints/BuildingCharacter.Ship Interact` _asbuilding_character (delegate `Enable Ship`)))

(event `Enable Ship`
  (`Controller.Possess` (`GameplayStatics.GetPlayerController` 0) self)
  (`self.SetActorHiddenInGame` (stale `self.ReceiveActorBeginOverlap` _asbuilding_character) true)
  (`self.SetActorHiddenInGame` (stale `self.ReceiveActorBeginOverlap` _output_get) true))

(event `self.ReceiveActorEndOverlap`
  (params (OtherActor :type "Actor Object Reference"))
  (bind _asbuilding_character (cast `/Game/PlayerBuildingSystem/Blueprints/BuildingCharacter` OtherActor))
  (clear `/Game/PlayerBuildingSystem/Blueprints/BuildingCharacter.Ship Interact` _asbuilding_character))

(event `self.ReceivePossessed`
  (params (NewController :type "Controller Object Reference"))
  (`self.EnableInput` NewController null))

(event `Key|E`
  (params (Key :type "Key Structure"))
  (bind _player (`self.Player`))
  (:`Pressed`
    (`self.K2_SetActorTransform` (`self.Player`) (`SceneComponent.K2_GetComponentToWorld` (`self.Jump out`)) false false)
    (`Controller.Possess` (`GameplayStatics.GetPlayerController` 0) _player)
    (`self.SetActorHiddenInGame` _player false)))

(event `InputAxis|MoveForward`
  (params (AxisValue :type "Float (single-precision)"))
  (`self.AddMovementInput` (`self.GetActorForwardVector`) (* AxisValue 0.8)))

(event `Key|W`
  (params (Key :type "Key Structure"))
  (bind _thruster (`self.Thruster`))
  (:`Pressed`
    (`AudioComponent.Play` _thruster 0.0))
  (:`Released`
    (`AudioComponent.Stop` _thruster)))

(event `InputAxis|MoveRight`
  (params (AxisValue :type "Float (single-precision)"))
  (`self.K2_AddActorLocalRotation` (`KismetMathLibrary.MakeRotator` 0.0 0.0 (* AxisValue 0.8))))

(fn `UserConstructionScript`)