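; BP_Item is a spawner that periodically launches OilResource actors toward an EndSpot actor.
; A looping timer started on BeginPlay spawns each resource at the spawner's root transform, with Y randomized between the root's Y and a fixed world coordinate.
; Each new resource's mesh receives a mass-independent velocity-change impulse along the look-at direction to EndSpot.
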(event `self.ReceiveBeginPlay`
  (`KismetSystemLibrary.K2_SetTimerDelegate` (delegate `SpawnItem`) 5.0 true))

(event `SpawnItem`
  (bind _returnvalue (`SceneComponent.K2_GetComponentToWorld` (`self.DefaultSceneRoot`)))
  (bind _returnvalue_2 (`|SpawnActorFromClass` "/Game/PlayerBuildingSystem/Blueprints/OilResource.OilResource_C" (`KismetMathLibrary.MakeTransform` (`KismetMathLibrary.MakeVector` (.x (.location _returnvalue)) (`KismetMathLibrary.RandomFloatInRange` (.y (.location _returnvalue)) 3000.0) (.z (.location _returnvalue))) (.rotation _returnvalue) (.scale _returnvalue)) "Undefined" "OverrideRootScale" null null))
  (`PrimitiveComponent.AddImpulse` (`/Game/PlayerBuildingSystem/Blueprints/MasterResource.Resource Mesh` _returnvalue_2) (* (`KismetMathLibrary.Conv_RotatorToVector` (`KismetMathLibrary.FindLookAtRotation` (`SceneComponent.K2_GetComponentLocation` (`/Game/PlayerBuildingSystem/Blueprints/MasterResource.Resource Mesh` _returnvalue_2)) (`self.K2_GetActorLocation` (`self.EndSpot`)))) (1000.0 1000.0 1000.0)) "None" true))

(fn `UserConstructionScript`)