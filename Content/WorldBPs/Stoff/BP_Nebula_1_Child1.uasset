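; Child Blueprint of BP_Nebula_1, a nebula world actor that drifts once when play begins and then removes its plane.
; After the parent BeginPlay, MoveComponentTo slides the root toward a fixed, distant relative location over a random duration of a few minutes.
; The Plane component is destroyed after the move node, with no Tick logic involved.
; The construction script only calls the parent.
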(event `self.ReceiveBeginPlay`
  (`parent.ReceiveBeginPlay`)
  (`KismetSystemLibrary.MoveComponentTo` (`self.DefaultSceneRoot`) (-20000.0 0.0 -10000.0) (struct) false false (`KismetMathLibrary.RandomFloatInRange` 150.0 200.0))
  (`ActorComponent.K2_DestroyComponent` (`self.Plane`))
  (`ActorComponent.K2_DestroyComponent` (`self.Plane`)))

(fn `UserConstructionScript`
  (`parent.UserConstructionScript`))