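; Nebula spawner actor that keeps at most one live nebula of its own in the world.
; A looping timer from BeginPlay calls TrySpawn, which spawns only when NebulaAmountOk is set and the last spawned nebula is no longer valid.
; SpawnItem picks a random class from NebulasToSpawn, placing it at a random Y offset from the spawner with random X/Y stretch.
; The NebulaAmount cap check is disconnected and never runs.
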(event `self.ReceiveBeginPlay`
  (`KismetSystemLibrary.K2_SetTimerDelegate` (delegate `Spawn nebula`) 10.0 true))

(event `Spawn nebula`
  (`self.TrySpawn`))

(fn `Spawn Item`
  (locals (NewLocalVar_0 :type "Transform Structure"))
  (bind (_returnvalue_x _returnvalue_y _returnvalue_z) (`KismetMathLibrary.BreakVector` (`self.K2_GetActorLocation`)))
  (bind (_returnvalue_roll _returnvalue_pitch _returnvalue_yaw) (`KismetMathLibrary.BreakRotator` (`self.K2_GetActorRotation`)))
  (bind _returnvalue (+ 1.0 (`KismetMathLibrary.RandomFloatInRange` 1.0 10.0)))
  (set `self.StoredTransform` (`self.GetTransform`))
  (bind _output_get (set `self.SpawnTransform` (`KismetMathLibrary.MakeTransform` (`KismetMathLibrary.MakeVector` _returnvalue_x (+ _returnvalue_y (`KismetMathLibrary.RandomFloatInRange` -30000.0 30000.0)) _returnvalue_z) (`KismetMathLibrary.MakeRotator` _returnvalue_roll _returnvalue_pitch _returnvalue_yaw) (`KismetMathLibrary.MakeVector` _returnvalue _returnvalue 1.0))))
  (bind _returnvalue_2 (`|SpawnActorFromClass` (`|GetArrayItem` (`self.NebulasToSpawn`) (`KismetMathLibrary.RandomIntegerInRange` 0 3)) _output_get "AlwaysSpawn" "OverrideRootScale" null null))
  (set `self.CurrentNebula` _returnvalue_2)
  (set `self.SpawnTransform` (`self.StoredTransform`)))

(fn `TrySpawn`
  (if (`self.Nebula Amount ok`)
    (`/Engine/EditorBlueprintResources/StandardMacros.IsValid` (`self.CurrentNebula`)
      (:`Is Not Valid`
        (`self.Spawn Item`)))))

(fn `UserConstructionScript`)